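; BP_Laser is a laser emitter Blueprint that fires a straight Cascade beam out of its Cube component.
; On Tick, a DoOnce spawns the P_Laser particle system attached to the Cube and caches it as LaserParticle.
; Each tick then sets the beam source to the Cube's location and its end point a fixed distance along the Cube's forward vector, with no trace or hit detection.
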(event EventTick
  (params (DeltaSeconds :type Float%20%28single-precision%29))
  (bind _cube (Variables|Default|GetCube))
  (bind _returnvalue (Transformation|GetWorldLocation _cube))
  (Utilities|FlowControl|Sequence
    (:then_0
      (Utilities|FlowControl|DoOnce false
        (:Completed
          (bind _returnvalue_2 (Effects|SpawnEmitterAttached "/Game/Models/Lazer/P_Laser.P_Laser" (Variables|Default|GetCube) "None"))
          (Variables|Default|SetLaser%20Particle _returnvalue_2))))
    (:then_1
      (Class|ParticleSystemComponent|SetBeamSourcePoint (Variables|Default|GetLaser%20Particle) 0 _returnvalue)
      (Class|ParticleSystemComponent|SetBeamEndPoint (Variables|Default|GetLaser%20Particle) 0 (+ _returnvalue (* (Math|Vector|GetForwardVector _cube) 5e+03))))))

(fn ConstructionScript)