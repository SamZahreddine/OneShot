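; BP_Laser is a laser hazard that kills the heroine character on contact.
; On the first tick it attaches a P_Laser beam particle to its Cube, then every tick stretches the beam from the cube a fixed distance along its forward vector.
; An overlap on the separate Collision component destroys Female_Heroine_BP, adds the Death widget to the viewport and shows the mouse cursor.
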(event OnComponentBeginOverlap(collision)
  (params (OverlappedComponent :type Primitive%20Component%20Object%20Reference) (OtherActor :type Actor%20Object%20Reference) (OtherComp :type Primitive%20Component%20Object%20Reference) (OtherBodyIndex :type Integer) (bFromSweep :type Boolean) (SweepResult :type Hit%20Result%20Structure%20%28by%20ref%29))
  ;[0 1 0.1562] if collided, die
  (bind _asfemale_heroine_bp (Utilities|Casting|CastToFemale_Heroine_BP OtherActor))
  (Actor|DestroyActor _asfemale_heroine_bp)
  (bind _returnvalue (UserInterface|CreateWidget "/Game/UI/Death.Death_C"))
  (UserInterface|Viewport|AddtoViewport _returnvalue 0)
  (Variables|/Script/Engine.PlayerController|SetbShowMouseCursor (Game|GetPlayerController 0) true))

(event EventTick
  (params (DeltaSeconds :type Float%20%28single-precision%29))
  (bind _cube (Variables|Default|GetCube))
  (bind _returnvalue (Transformation|GetWorldLocation _cube))
  ;[0.3359 1 0] spawn particle
  (Utilities|FlowControl|Sequence
    (:then_0
      (Utilities|FlowControl|DoOnce false
        (:Completed
          (bind _returnvalue_2 (Effects|SpawnEmitterAttached "/Game/Models/Laser/P_Laser.P_Laser" (Variables|Default|GetCube) "None"))
          (Variables|Default|SetLaser%20Particle _returnvalue_2))))
    (:then_1
      (Class|ParticleSystemComponent|SetBeamSourcePoint (Variables|Default|GetLaser%20Particle) 0 _returnvalue)
      (Class|ParticleSystemComponent|SetBeamEndPoint (Variables|Default|GetLaser%20Particle) 0 (+ _returnvalue (* (Math|Vector|GetForwardVector _cube) 5e+03))))))

(fn ConstructionScript)